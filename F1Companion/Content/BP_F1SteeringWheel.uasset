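; F1 steering wheel actor that animates its PivotSterzo component from telemetry supplied by the TelemetryManager game instance.
; Each new location timestamp turns the normalized yaw change into an amplified target angle, so steering is estimated from heading change.
; Every tick the pivot's roll eases toward that angle.
; Brake minus throttle also nudges the pivot's position, smoothed through rotator interpolation whose roll and pitch become X and Y.
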(event `self.ReceiveBeginPlay`
  (bind _astelemetry_manager (cast `TelemetryManager` (`GameplayStatics.GetGameInstance`)))
  (set `self.Ref_Telemetry` _astelemetry_manager))

(event `self.ReceiveTick`
  (params (DeltaSeconds :type "Float (single-precision)"))
  (bind _pivotsterzo (`self.PivotSterzo`))
  (bind _ref_telemetry (`self.Ref_Telemetry`))
  (bind (_x_coor _y_coor _yaw _z_coor _timestamp) (break `LocationData` (`TelemetryManager.CurrentLocation` _ref_telemetry)))
  (bind (_gear _speed _rpm _throttle _brake) (break `VehicleTelemetryData` (`TelemetryManager.CurrentTelemetry` _ref_telemetry)))
  (bind _returnvalue_roll (`KismetMathLibrary.BreakRotator` (`KismetMathLibrary.RInterpTo` (`SceneComponent.RelativeRotation` _pivotsterzo) (`KismetMathLibrary.MakeRotator` (`self.AngoloTarget`)) DeltaSeconds 5.0)))
  (bind (_returnvalue_roll_2 _returnvalue_pitch) (`KismetMathLibrary.BreakRotator` (`KismetMathLibrary.RInterpTo` (`KismetMathLibrary.Conv_VectorToRotator` (`SceneComponent.RelativeLocation` _pivotsterzo)) (`KismetMathLibrary.MakeRotator` (- (* _brake 0.05) (* (`KismetMathLibrary.Conv_IntToDouble` _throttle) 0.05))) DeltaSeconds 10.0)))
  (if (`KismetStringLibrary.NotEqual_StrStr` _timestamp (`self.UltimoTimestamp`))
    (set `self.AngoloTarget` (* (`KismetMathLibrary.NormalizeAxis` (- _yaw (`self.YawPrecedente`))) 12.0))
    (set `self.YawPrecedente` _yaw)
    (set `self.UltimoTimestamp` _timestamp))
  (`SceneComponent.K2_SetRelativeRotation` _pivotsterzo (`KismetMathLibrary.MakeRotator` _returnvalue_roll) false false)
  (`SceneComponent.K2_SetRelativeLocation` _pivotsterzo (`KismetMathLibrary.MakeVector` _returnvalue_roll_2 _returnvalue_pitch) false false))

(fn `UserConstructionScript`)